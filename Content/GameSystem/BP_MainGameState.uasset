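; Main game state Blueprint that, as a debug shortcut, unlocks social classes for the city at game start.
; BeginPlay runs a three-branch Sequence, one per wealth tier (Poor, Middle, Rich), each calling UnlockSocialClass after a short Delay with a uniform default demand.
; Poor and Middle unlock Finance, Science, Tourism, Military and Spiritual specialties, while Rich omits Finance.
; Tick and the construction script are empty.
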(event EventBeginPlay
  (bind _returnvalue (Utilities|Enum|LiteralenumEWealthLevels "Rich"))
  (bind _returnvalue_2 (Utilities|Enum|LiteralenumEWealthLevels "Middle"))
  (bind _returnvalue_3 (Utilities|Enum|LiteralenumEWealthLevels "Poor"))
  ;[1 0 0] DEBUG Unlock all Classes
  (Utilities|FlowControl|Sequence
    (:then_0
      ;;[1 1 1] Poor Classes
      (Utilities|FlowControl|Delay 0.2)
      (Class|MainGameState|UnlockSocialClass _returnvalue_3 (Utilities|Enum|LiteralenumECitySpecialty "Finance") 0.5)
      (Class|MainGameState|UnlockSocialClass _returnvalue_3 (Utilities|Enum|LiteralenumECitySpecialty "Science") 0.5)
      (Class|MainGameState|UnlockSocialClass _returnvalue_3 (Utilities|Enum|LiteralenumECitySpecialty "Tourism") 0.5)
      (Class|MainGameState|UnlockSocialClass _returnvalue_3 (Utilities|Enum|LiteralenumECitySpecialty "Military") 0.5)
      (Class|MainGameState|UnlockSocialClass _returnvalue_3 (Utilities|Enum|LiteralenumECitySpecialty "Spiritual") 0.5))
    (:then_1
      ;;[1 1 1] Middle Classes
      (Utilities|FlowControl|Delay 0.2)
      (Class|MainGameState|UnlockSocialClass _returnvalue_2 (Utilities|Enum|LiteralenumECitySpecialty "Finance") 0.5)
      (Class|MainGameState|UnlockSocialClass _returnvalue_2 (Utilities|Enum|LiteralenumECitySpecialty "Science") 0.5)
      (Class|MainGameState|UnlockSocialClass _returnvalue_2 (Utilities|Enum|LiteralenumECitySpecialty "Tourism") 0.5)
      (Class|MainGameState|UnlockSocialClass _returnvalue_2 (Utilities|Enum|LiteralenumECitySpecialty "Military") 0.5)
      (Class|MainGameState|UnlockSocialClass _returnvalue_2 (Utilities|Enum|LiteralenumECitySpecialty "Spiritual") 0.5))
    (:then_2
      ;;[1 1 1] Rich Classes
      (Utilities|FlowControl|Delay 0.2)
      (Class|MainGameState|UnlockSocialClass _returnvalue (Utilities|Enum|LiteralenumECitySpecialty "Science") 0.5)
      (Class|MainGameState|UnlockSocialClass _returnvalue (Utilities|Enum|LiteralenumECitySpecialty "Tourism") 0.5)
      (Class|MainGameState|UnlockSocialClass _returnvalue (Utilities|Enum|LiteralenumECitySpecialty "Military") 0.5)
      (Class|MainGameState|UnlockSocialClass _returnvalue (Utilities|Enum|LiteralenumECitySpecialty "Spiritual") 0.5))))

(event EventTick
  (params (DeltaSeconds :type Float%20%28single-precision%29)))

(fn ConstructionScript)
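; Player controller for a city-building game that creates the HUD widgets and handles clicks on the world.
; A cursor trace uses actor tags to show the construction widget for empty slots or the info widget for buildings.
; A validated construction event spawns the chosen class from the GameMode's buildings map, registers it with the GameState and destroys the slot.
; Debug inputs adjust satisfaction and residential demand; the menu toggle logic is disconnected.
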(event Custom|ED%20Building%20Construction%20Validated_Event
  (params (BuildingName :type Name))
  (bind _last_constructible_slot (Variables|Default|GetLast%20Constructible%20Slot))
  (bind _last_constructible_slot_2 (Variables|Default|GetLast%20Constructible%20Slot))
  (bind _as_bp_main_game_mode (Variables|Default|GetAs%20BP%20Main%20Game%20Mode))
  (bind _returnvalue (Class|ConstructibleSlot|GetSlotType _last_constructible_slot_2))
  (bind _returnvalue_2 (Class|ConstructibleSlot|GetSlotSize _last_constructible_slot_2))
  (bind _returnvalue_3 (Class|MainGameMode|GetBuildingsMap _as_bp_main_game_mode _returnvalue _returnvalue_2))
  (bind (_value _returnvalue_4) (Utilities|Map|Find _returnvalue_3 BuildingName))
  ;[1 1 1] GESTION ED_BuildingConstructionValidate
  (Development|PrintString (Utilities|String|ToString(Name) BuildingName))
  (CallFunction|HideAllWidgets)
  (if (Utilities|IsValid (Variables|Default|GetLast%20Constructible%20Slot))
    (if _returnvalue_4
      (if (Utilities|IsValidClass (.building _value))
        (bind _returnvalue_5 (Game|SpawnActorfromClass (.building _value) (Math|Transform|MakeTransform (Transformation|GetActorLocation _last_constructible_slot_2) (Transformation|GetActorRotation _last_constructible_slot_2) "1,1,1") "Undefined" 0 0))
        (Utilities|FlowControl|Sequence
          (:then_0
            (Class|MainGameState|AddNewBuilding (Variables|Default|GetAs%20Main%20Game%20State) _returnvalue_5))
          (:then_1
            (bind _asresidential_building (Utilities|Casting|CastToResidentialBuilding _returnvalue_5))
            (switch Utilities|FlowControl|Switch|SwitchonESlotSize (Class|ConstructibleSlot|GetSlotSize _last_constructible_slot)
              (:Small
                (Variables|/Script/LittleBigTown.ResidentialBuilding|Set_DistancePedestrianSpawn _asresidential_building 250))
              (:Medium
                (Variables|/Script/LittleBigTown.ResidentialBuilding|Set_DistancePedestrianSpawn _asresidential_building 350))
              (:Large
                (Variables|/Script/LittleBigTown.ResidentialBuilding|Set_DistancePedestrianSpawn _asresidential_building 400))))
          (:then_2
            (Class|Building|SetDistrictName _returnvalue_5 (Class|ConstructibleSlot|GetDistrictName _last_constructible_slot))
            (Actor|DestroyActor _last_constructible_slot))))
      (else
        (Development|PrintString "Error in BP MainPlayerController : Key not found in buildings map")))))

(event EventBeginPlay
  (Utilities|FlowControl|Sequence
    (:then_0
      (bind _asbp_main_game_mode (Utilities|Casting|CastToBP_MainGameMode (Game|GetGameMode))
        (:then
          (Variables|Default|SetAs%20BP%20Main%20Game%20Mode _asbp_main_game_mode)
          (bind _asmain_game_state (Utilities|Casting|CastToMainGameState (Game|GetGameState))
            (:then
              (Variables|Default|SetAs%20Main%20Game%20State _asmain_game_state))
            (:CastFailed
              (Development|PrintString "BP_BGMainPlayerController : Error, Cast BP Game State Failed."))))
        (:CastFailed
          (Development|PrintString "BP_BGMainPlayerController : Error, Cast BP Game Mode Failed."))))
    (:then_1
      ;[1 1 1] Creating Thematic Building Widgets
      (bind _returnvalue (UserInterface|CreateWidget "/Game/GameSystem/UserInterface/UI_Graphs/BP_WIdgetGraphs.BP_WidgetGraphs_C" self))
      (UserInterface|Viewport|AddtoViewport _returnvalue 0)
      (bind _returnvalue_2 (UserInterface|CreateWidget "/Game/GameSystem/UserInterface/UI_Main/BP_WidgetMainInteface.BP_WidgetMainInteface_C" self))
      (UserInterface|Viewport|AddtoViewport _returnvalue_2 0)
      (bind _returnvalue_3 (UserInterface|CreateWidget "/Game/GameSystem/UserInterface/UI_BuildingInfos/BP_Widget_BuildingInfos.BP_Widget_BuildingInfos_C" self))
      (UserInterface|Viewport|AddtoViewport _returnvalue_3 0)
      (bind _returnvalue_4 (UserInterface|CreateWidget "/Game/GameSystem/UserInterface/UI_Construction/BP_WidgetConstruction.BP_WidgetConstruction_C"))
      (UserInterface|Viewport|AddtoViewport _returnvalue_4 0))
    (:then_2
      ;[1 1 1] GESTION ED_BuildingConstructionValidate
      (EventDispatchers|BindEventtoEDBuildingConstructionValidated (delegate Custom|ED%20Building%20Construction%20Validated_Event)))))

(event EventTick
  (params (DeltaSeconds :type Float%20%28single-precision%29)))

(event Input|ActionEvents|InputActionOpenMenu
  (params (Key :type Key%20Structure :default "None"))
  ;[0 0.527 1] Open/Close Menu
)

(event Input|ActionEvents|InputActionMouseClick
  (params (Key :type Key%20Structure :default "None"))
  (bind (_hitresult _returnvalue) (Game|Player|GetHitResultUnderCursorbyChannel "TraceTypeQuery1" true))
  ;[1 0.2983 0] GESTION CLICKS EVENTS
  (:Pressed
    (if (Variables|Default|GetbEnableClickEvents)
      (if _returnvalue
        (bind _output_get (Variables|Default|SetHit%20Result%20Hit%20Actor (.hitactor _hitresult)))
        (Utilities|Casting|CastToPedestrian _output_get
          (:then
            (Development|PrintString "Pedestrian"))
          (:CastFailed
            (Development|PrintString (Utilities|GetDisplayName (Variables|Default|GetHit%20Result%20Hit%20Actor)))))
        (CallFunction|HideAllWidgets)
        (if (Actor|ActorHasTag (Variables|Default|GetHit%20Result%20Hit%20Actor) "ConstructibleSlot")
          (bind _asconstructible_slot (Utilities|Casting|CastToConstructibleSlot (Variables|Default|GetHit%20Result%20Hit%20Actor))
            (:then
              (CallFunction|ConstructibleSlotClickInteract _asconstructible_slot))
            (:CastFailed
              (Development|PrintString "Error : Object has tag \"ConstructibleSlot\" but cannot be cast to ConstructibleSlot Type.")))
          (elif (Actor|ActorHasTag (Variables|Default|GetHit%20Result%20Hit%20Actor) "Building")
            (bind _asbuilding (Utilities|Casting|CastToBuilding (Variables|Default|GetHit%20Result%20Hit%20Actor))
              (:then
                (Variables|Default|SetDEBUGLastBuilding _asbuilding)
                (Class|UIBuildingInfos|NewDisplayBuildingInfos (Variables|Default|Get_BuildingInfosWidget) _asbuilding))
              (:CastFailed
                (Development|PrintString "Error : Object has tag \"Building\" but cannot be cast to Building Type.")))))))))

(event Input|ActionEvents|InputActionADDSATISFACTIONDEBUG
  (params (Key :type Key%20Structure :default "None"))
  ;[1 0 0.02002] DEBUGG
  (:Pressed
    (bind _asresidential_building (Utilities|Casting|CastToResidentialBuilding (Variables|Default|GetDEBUGLastBuilding))
      (:then
        (Class|ResidentialBuilding|AddSatisfaction _asresidential_building 0.1))
      (:CastFailed
        (Development|PrintString "NOT A RESIDENTIAL BUILDING")))))

(event Input|ActionEvents|InputActionSUBSATISFACTIONDEBUG
  (params (Key :type Key%20Structure :default "None"))
  ;[1 0 0.02002] DEBUGG
  (:Pressed
    (bind _asresidential_building (Utilities|Casting|CastToResidentialBuilding (Variables|Default|GetDEBUGLastBuilding))
      (:then
        (Class|ResidentialBuilding|AddSatisfaction _asresidential_building -0.1))
      (:CastFailed
        (Development|PrintString "NOT A RESIDENTIAL BUILDING")))))

(event Input|ActionEvents|InputActionPOS_NEG_DEMAND_SWITCH
  (params (Key :type Key%20Structure :default "None"))
  (bind _as_main_game_state (Variables|Default|GetAs%20Main%20Game%20State))
  ;[1 0 0.02002] DEBUGG
  (:Pressed
    (Utilities|FlowControl|FlipFlop
      (:A
        (Class|MainGameState|DebugSetResidentialDemand _as_main_game_state 0.5 0.5 0.5))
      (:B
        (Class|MainGameState|DebugSetResidentialDemand _as_main_game_state -0.5 -0.5 -0.5)))))

(fn ConstructionScript)

(fn HideAllWidgets
  (Widget|SetVisibility (Variables|Default|Get_ConstructionWidget) "Collapsed")
  ;[1 0 0] Cette fonction supprime Delegate + weak object ptr du BuildingInfosWidget
  (Class|BGUserWidget|Hide (Variables|Default|Get_BuildingInfosWidget)))

(fn ConstructibleSlotClickInteract
  (params (ConstructibleSlot :type Constructible%20Slot%20Object%20Reference))
  (bind _output_get (Variables|Default|SetLast%20Constructible%20Slot ConstructibleSlot))
  (Class|UIConstructionMain|UpdateandDisplayInterface (Variables|Default|Get_ConstructionWidget) (Class|ConstructibleSlot|GetSlotType _output_get) (Class|ConstructibleSlot|GetSlotSize _output_get)))
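; Dynamic sky actor that moves the sun with the game's clock.
; On BeginPlay it binds to BP_MainGameState's new-hour and new-minute delegates and sets an initial pitch on the directional light.
; Each new minute it converts the stored hour and minute into fractional hours, samples a float curve for the light's pitch, then calls UpdateSunDirection to refresh the sky.
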(event Custom|OnNewHourDelegate_Event_0
  (params (Hour :type Integer))
  ;[1 1 1] Comment
  (Variables|Default|SetHours Hour))

(event Custom|OnNewMinuteDelegate_Event_0
  (params (Minute :type Integer))
  ;[1 1 1] Comment
  (Variables|Default|SetMinutes Minute)
  (Transformation|SetActorRotation (Variables|Default|GetDirectional%20light%20actor) (Math|Rotator|MakeRotator 0.0 (Math|Curves|GetFloatValue (Variables|Default|GetCurveFloat) (+ (Math|Conversions|ToFloat(Integer) (Variables|Default|GetHours)) (/ (Math|Conversions|ToFloat(Integer) (Variables|Default|GetMinutes)) 6e+01))) 0.0))
  (CallFunction|UpdateSunDirection))

(event EventBeginPlay
  ;[1 1 1] Comment
  (bind _asbp_main_game_state (Utilities|Casting|CastToBP_MainGameState (Game|GetGameState))
    (:then
      (EventDispatchers|AssignOnNewHourDelegate _asbp_main_game_state (delegate Custom|OnNewHourDelegate_Event_0))
      (EventDispatchers|AssignOnNewMinuteDelegate _asbp_main_game_state (delegate Custom|OnNewMinuteDelegate_Event_0))
      (Transformation|SetActorRotation (Variables|Default|GetDirectional%20light%20actor) (Math|Rotator|MakeRotator 0.0 9e+01 0.0)))
    (:CastFailed
      (Development|PrintString "Cast failed in BP_Level"))))

(event EventTick
  (params (DeltaSeconds :type Float%20%28single-precision%29)))

(fn ConstructionScript
  (|CallParentFunction))
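; Main player controller that sets up mouse input at game start and caches screen metrics.
; BeginPlay works around a cursor-jumps-to-top-left launch bug: it disables camera movement, waits briefly, centers the cursor, locks it to the viewport and shows it.
; MajScreenSize stores the viewport size and percentage-based border margins, skipping zero-sized viewports; it is meant to be called again when resolution settings change.
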(event EventBeginPlay
  (bind _screensize (Variables|Default|GetScreenSize))
  ;[0 0.8775 1] Toute cette merde (sauf MajScreenSize) sert à contrer le bug du curseur qui part en haut à gauche au lancement du jeu. Si on trouve moyen de contrer le bug autrement, il sera possible de tout supprimer.
  (Variables|Default|SetDisableCameraMovements true)
  (Utilities|FlowControl|Delay 1.0)
  ;;[1 0 0] To Call When Changing Res Settings !
  (CallFunction|MajScreenSize)
  (Class|PlayerController|SetMouseLocation (Math|Float|Truncate (/ (.x _screensize) 2.0)) (Math|Float|Truncate (/ (.y _screensize) 2.0)))
  (Input|SetInputModeGameandUI self 0 "LockAlways" false)
  (Variables|Default|SetbShowMouseCursor true)
  (Variables|Default|SetDisableCameraMovements false))

(event EventTick
  (params (DeltaSeconds :type Float%20%28single-precision%29)))

(fn ConstructionScript)

(fn MajScreenSize
  (bind (_sizex _sizey) (HUD|GetViewportSize))
  (bind _screenborderper (Variables|Default|GetScreenBorderPer))
  (bind _returnvalue (Math|Conversions|ToFloat(Integer) _sizex))
  (bind _returnvalue_2 (Math|Conversions|ToFloat(Integer) _sizey))
  (bind _returnvalue_3 (Math|Vector2D|MakeVector2D _returnvalue _returnvalue_2))
  (if (Math|Vector|NotEqual(Vector) :A _returnvalue_3 :ErrorTolerance 0.0)
    (Variables|Default|SetScreenSize _returnvalue_3)
    (Variables|Default|SetborderX (/ (* _screenborderper _returnvalue) 1e+02))
    (Variables|Default|SetborderY (/ (* _screenborderper _returnvalue_2) 1e+02))))